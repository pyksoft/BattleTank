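; Player-controllable tank Blueprint that binds input to aiming, driving and firing.
; On BeginPlay it passes its turret and barrel components to inherited or external setter functions.
; Aim axes rotate the azimuth gimbal and spring arm, scaled by frame time, to orbit the camera.
; Per-track throttle axes drive each track directly, a Forward axis feeds movement intent to TankMovementComponent, and the Fire action calls Fire.
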(event `self.ReceiveBeginPlay`
  (`self.SetTurretReference` (`self.TankTurret`))
  (`self.SetBarrelReference` (`self.TankBarrel`)))

(event `InputAxis|AimAzimuth`
  (params (AxisValue :type "Float (single-precision)"))
  ;[1 1 1] Camera Input binding
  (`SceneComponent.K2_AddLocalRotation` (`self.Azimuth Gimbal`) (`KismetMathLibrary.MakeRotator` 0.0 0.0 (* (`GameplayStatics.GetWorldDeltaSeconds`) AxisValue 100.0)) false false))

(event `InputAxis|Left Track Throttle`
  (params (AxisValue :type "Float (single-precision)"))
  ;[1 1 1] Movement Input Binding
  (`TankTrack.SetThrottle` (`self.LeftTrack`) AxisValue))

(event `InputAxis|AimElevation`
  (params (AxisValue :type "Float (single-precision)"))
  ;[1 1 1] Camera Input binding
  (`SceneComponent.K2_AddLocalRotation` (`self.SpringArm`) (`KismetMathLibrary.MakeRotator` 0.0 (* (`GameplayStatics.GetWorldDeltaSeconds`) AxisValue 100.0)) false false))

(event `InputAxis|Right Track Throttle`
  (params (AxisValue :type "Float (single-precision)"))
  ;[1 1 1] Movement Input Binding
  (`TankTrack.SetThrottle` (`self.RightTrack`) AxisValue))

(event `InputAction|Fire`
  (params (Key :type "Key Structure" :default "AnyKey"))
  ;[1 1 1] Camera Input binding
  (:`Pressed`
    (`self.Fire`)))

(event `InputAxis|Forward`
  (params (AxisValue :type "Float (single-precision)"))
  ;[1 1 1] Movement Input Binding
  (`TankMovementComponent.IntendMoveForward` (`self.TankMovementComponent`) AxisValue))

(fn `UserConstructionScript`)